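; Base Blueprint for a player-driven sports vehicle with an orbiting spring-arm camera.
; On BeginPlay it adds the vehicle Enhanced Input mapping context to the local player.
; Throttle, brake, steering and handbrake actions pass their values straight to the vehicle movement component, including on release.
; Look input rotates the spring arm, then a helper clamps pitch and yaw and zeroes roll to limit the view.
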(event Input|EnhancedActionEvents|EnhancedInputActionIA_LookAround
  (params (ActionValue :type Vector%202D%20Structure) (ElapsedSeconds :type Float%20%28double-precision%29) (TriggeredSeconds :type Float%20%28double-precision%29) (InputAction :type Input%20Action%20Object%20Reference :default "/Game/Blueprints/Vehicles/Input/IA_LookAround.IA_LookAround"))
  (bind (_x _y) (Math|Vector2D|BreakVector2D ActionValue))
  (bind _springarm (Variables|Default|GetSpringArm))
  ;[0 0 0] Movement
  (Transformation|AddLocalRotation _springarm (Math|Rotator|MakeRotator 0.0 _y _x) false false)
  (Transformation|SetRelativeRotation _springarm (CallFunction|GetSpringArmRelativeRotaion) false false))

(event Input|EnhancedActionEvents|EnhancedInputActionIA_Throttle
  (params (ActionValue :type Float%20%28double-precision%29) (ElapsedSeconds :type Float%20%28double-precision%29) (TriggeredSeconds :type Float%20%28double-precision%29) (InputAction :type Input%20Action%20Object%20Reference :default "/Game/Blueprints/Vehicles/Input/IA_Throttle.IA_Throttle"))
  ;[0 0 0] Movement
  (:Triggered
    (Class|ChaosVehicleMovementComponent|SetThrottleInput (Variables|Default|GetVehicleMovementComponent) ActionValue :!label _label))
  (:Started
    (goto _label))
  (:Completed
    (goto _label)))

(event Input|EnhancedActionEvents|EnhancedInputActionIA_Brake
  (params (ActionValue :type Float%20%28double-precision%29) (ElapsedSeconds :type Float%20%28double-precision%29) (TriggeredSeconds :type Float%20%28double-precision%29) (InputAction :type Input%20Action%20Object%20Reference :default "/Game/Blueprints/Vehicles/Input/IA_Brake.IA_Brake"))
  ;[0 0 0] Movement
  (:Triggered
    (Class|ChaosVehicleMovementComponent|SetBrakeInput (Variables|Default|GetVehicleMovementComponent) ActionValue :!label _label))
  (:Started
    (goto _label))
  (:Completed
    (goto _label)))

(event Input|EnhancedActionEvents|EnhancedInputActionIA_Steering
  (params (ActionValue :type Float%20%28double-precision%29) (ElapsedSeconds :type Float%20%28double-precision%29) (TriggeredSeconds :type Float%20%28double-precision%29) (InputAction :type Input%20Action%20Object%20Reference :default "/Game/Blueprints/Vehicles/Input/IA_Steering.IA_Steering"))
  ;[0 0 0] Movement
  (:Triggered
    (Class|ChaosVehicleMovementComponent|SetSteeringInput (Variables|Default|GetVehicleMovementComponent) ActionValue :!label _label))
  (:Started
    (goto _label))
  (:Completed
    (goto _label)))

(event Input|EnhancedActionEvents|EnhancedInputActionIA_Handbrake
  (params (ActionValue :type Boolean) (ElapsedSeconds :type Float%20%28double-precision%29) (TriggeredSeconds :type Float%20%28double-precision%29) (InputAction :type Input%20Action%20Object%20Reference :default "/Game/Blueprints/Vehicles/Input/IA_Handbrake.IA_Handbrake"))
  ;[0 0 0] Movement
  (:Triggered
    (Class|ChaosVehicleMovementComponent|SetHandbrakeInput (Variables|Default|GetVehicleMovementComponent) ActionValue :!label _label))
  (:Started
    (goto _label))
  (:Ongoing
    (goto _label))
  (:Canceled
    (goto _label))
  (:Completed
    (goto _label)))

(event EventBeginPlay
  (bind _asplayer_controller (Utilities|Casting|CastToPlayerController (Pawn|GetController)))
  (Utilities|IsValid (PlayerController|LocalPlayerSubsystems|GetEnhancedInputLocalPlayerSubsystem _asplayer_controller)
    (:Is%20Valid
      (Input|AddMappingContext (PlayerController|LocalPlayerSubsystems|GetEnhancedInputLocalPlayerSubsystem _asplayer_controller) (Variables|Default|GetVehiceMappingContext) 0 "(bIgnoreAllPressedKeysUntilRelease=True,bForceImmediately=False,bNotifyUserSettings=False)"))))

(fn ConstructionScript)

(fn GetSpringArmRelativeRotaion
  (bind _springarm (Variables|Default|GetSpringArm))
  (bind _relativerotation (Variables|/Script/Engine.SceneComponent|GetRelativeRotation _springarm))
  (return (Math|Rotator|MakeRotator 0.0 (Math|Float|ClampAngle (.pitch _relativerotation) -5e+01 0.0) (Math|Float|ClampAngle (.yaw _relativerotation) -1.2e+02 1.2e+02))))