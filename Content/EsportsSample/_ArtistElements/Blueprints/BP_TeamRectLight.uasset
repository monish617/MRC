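; Team-colored rect light actor for the esports sample, tinted with Team A or Team B light color.
; Exposed variables drive intensity, attenuation, source size, barn doors, shadows, visibility, lighting channels and ray-tracing options.
; Color comes from the MPC_TeamColorController material parameter collection, chosen by the Team enum.
; The Construction Script and BeginPlay apply identical setup, with color read once each run rather than updated continuously.
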(event EventBeginPlay
  (bind _rectlight (Variables|Default|GetRectLight))
  (Rendering|Components|Light|SetIntensity _rectlight (Variables|LightProperties|GetLight%20Intensity))
  (Rendering|Lighting|SetAttenuationRadius _rectlight (Variables|LightProperties|GetAttenuation%20Radius))
  (Class|RectLightComponent|SetSourceWidth _rectlight (Variables|LightProperties|GetWidth))
  (Class|RectLightComponent|SetSourceHeight _rectlight (Variables|LightProperties|GetHeight))
  (Class|RectLightComponent|SetBarnDoorAngle _rectlight (Variables|LightProperties|GetBarn%20Door%20Angle))
  (Class|RectLightComponent|SetBarnDoorLength _rectlight (Variables|LightProperties|GetBarn%20Door%20Height))
  (Rendering|Components|Light|SetCastShadows _rectlight (Variables|LightProperties|GetCast%20Shadows))
  (Rendering|SetVisibility _rectlight (Variables|LightProperties|GetVisibility) true)
  (Rendering|Components|SetLightingChannels _rectlight (Variables|LightProperties|GetLighting%20Channel%200) (Variables|LightProperties|GetLighting%20Channel%201) (Variables|LightProperties|GetLighting%20Channel%202))
  (Class|LightComponentBase|SetCastRaytracedShadow _rectlight (Variables|LightProperties|GetCast%20RT%20Shadows))
  (Class|LightComponentBase|SetAffectReflection _rectlight (Variables|LightProperties|GetCast%20RT%20Reflections))
  (if (Utilities|Enum|Equal(Enum) (Variables|Default|GetTeam) "NewEnumerator0")
    (bind _returnvalue (Rendering|Material|GetVectorParameterValue "/Game/EsportsSample/_ArtistElements/Materials/Collections/MPC_TeamColorController.MPC_TeamColorController" "TeamALight" :!class /Script/Engine.KismetMaterialLibrary))
    (Rendering|Components|Light|SetLightColor (Variables|Default|GetRectLight) _returnvalue true)
    (else
      (bind _returnvalue_2 (Rendering|Material|GetVectorParameterValue "/Game/EsportsSample/_ArtistElements/Materials/Collections/MPC_TeamColorController.MPC_TeamColorController" "TeamBLight" :!class /Script/Engine.KismetMaterialLibrary))
      (Rendering|Components|Light|SetLightColor (Variables|Default|GetRectLight) _returnvalue_2 true))))

(fn ConstructionScript
  (bind _rectlight (Variables|Default|GetRectLight))
  (Rendering|Components|Light|SetIntensity _rectlight (Variables|LightProperties|GetLight%20Intensity))
  (Rendering|Lighting|SetAttenuationRadius _rectlight (Variables|LightProperties|GetAttenuation%20Radius))
  (Class|RectLightComponent|SetSourceWidth _rectlight (Variables|LightProperties|GetWidth))
  (Class|RectLightComponent|SetSourceHeight _rectlight (Variables|LightProperties|GetHeight))
  (Class|RectLightComponent|SetBarnDoorAngle _rectlight (Variables|LightProperties|GetBarn%20Door%20Angle))
  (Class|RectLightComponent|SetBarnDoorLength _rectlight (Variables|LightProperties|GetBarn%20Door%20Height))
  (Rendering|Components|Light|SetCastShadows _rectlight (Variables|LightProperties|GetCast%20Shadows))
  (Rendering|SetVisibility _rectlight (Variables|LightProperties|GetVisibility) true)
  (Rendering|Components|SetLightingChannels _rectlight (Variables|LightProperties|GetLighting%20Channel%200) (Variables|LightProperties|GetLighting%20Channel%201) (Variables|LightProperties|GetLighting%20Channel%202))
  (Class|LightComponentBase|SetCastRaytracedShadow _rectlight (Variables|LightProperties|GetCast%20RT%20Shadows))
  (Class|LightComponentBase|SetAffectReflection _rectlight (Variables|LightProperties|GetCast%20RT%20Reflections))
  (if (Utilities|Enum|Equal(Enum) (Variables|Default|GetTeam) "NewEnumerator0")
    (bind _returnvalue (Rendering|Material|GetVectorParameterValue "/Game/EsportsSample/_ArtistElements/Materials/Collections/MPC_TeamColorController.MPC_TeamColorController" "TeamALight" :!class /Script/Engine.KismetMaterialLibrary))
    (Rendering|Components|Light|SetLightColor (Variables|Default|GetRectLight) _returnvalue true)
    (else
      (bind _returnvalue_2 (Rendering|Material|GetVectorParameterValue "/Game/EsportsSample/_ArtistElements/Materials/Collections/MPC_TeamColorController.MPC_TeamColorController" "TeamBLight" :!class /Script/Engine.KismetMaterialLibrary))
      (Rendering|Components|Light|SetLightColor (Variables|Default|GetRectLight) _returnvalue_2 true))))