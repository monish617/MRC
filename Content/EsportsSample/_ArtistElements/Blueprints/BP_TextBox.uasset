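; BP_TextBox is an esports sample actor that pairs 3D text with a backing plane sized to fit it.
; Its construction script calls ApplyDesign, which copies the actor bounds into a box component, then scales the plane from that extent plus padding.
; The plane gets the text box material, with its slant parameter scaled by padded height.
; SetText styles the text but is not called here; an older three-mesh approach is disconnected.
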(event Custom|Apply%20Design
  (bind _padding_topbot (Variables|Default|GetPadding_TopBot))
  (bind _box (Variables|Default|GetBox))
  (bind _returnvalue (Components|Box|GetScaledBoxExtent _box))
  (bind (_x _y _z) (Math|Vector|BreakVector _returnvalue))
  (bind _returnvalue_2 (+ _z _padding_topbot))
  (bind _returnvalue_3 (* _returnvalue_2 0.02))
  (Utilities|FlowControl|Sequence
    (:then_1
      ;[0 0 0] Set Box Extent
      (Components|Box|SetBoxExtent _box (.BoxExtent (Collision|GetActorBounds false false)) true)
      (Variables|Default|SetBounds%20Size _returnvalue))
    (:then_2
      ;[0 0 0] Set new dimensions on plane
      (Transformation|SetWorldScale3D (Variables|Default|GetPlane) (Math|Vector|MakeVector (* (+ _x (Variables|Default|GetPadding_LeftRight)) 0.02) _returnvalue_3 1.0)))
    (:then_3
      ;[0 0 0] Set Materials + Set slant amount dynamically
      (Rendering|Material|SetMaterial (Variables|Default|GetPlane) 0 (Variables|Default|GetText%20Box%20Material))
      (Rendering|Material|SetScalarParameterValueonMaterials (Variables|Default|GetPlane) "Slant Amount" (* (Variables|Default|GetSlant%20Amount) _returnvalue_3)))
    (:then_4)))

(fn ConstructionScript
  (CallFunction|ApplyDesign))