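; Logo actor for the Esports sample that displays an assignable texture on its SMLogo mesh component.
; The construction script calls UpdateTexture, which creates a dynamic instance of MI_HexLogo_URL for material slot 2.
; It sets the Diffuse parameter from the TextureSlot variable and applies the instance to that slot.
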(event Custom|UpdateTexture
  (bind _returnvalue (Rendering|Material|CreateDynamicMaterialInstance (Variables|Default|GetSM_Logo) 2 "/Game/EsportsSample/_TeamElements/Materials/MI_HexLogo_URL.MI_HexLogo_URL" "None" :!class /Script/Engine.PrimitiveComponent))
  (Rendering|Material|SetTextureParameterValue _returnvalue "Diffuse" (Variables|Default|GetTextureSlot))
  (Rendering|Material|SetMaterial (Variables|Default|GetSM_Logo) 2 _returnvalue))

(event EventBeginPlay
  (|CallParentFunction) ; This node is disabled and will not be called.\nDrag off pins to build functionality.
)

(event Collision|EventActorBeginOverlap
  (params (OtherActor :type Actor%20Object%20Reference)))

(event EventTick
  (params (DeltaSeconds :type Float%20%28single-precision%29)))

(fn ConstructionScript
  (|CallParentFunction)
  (CallFunction|UpdateTexture))