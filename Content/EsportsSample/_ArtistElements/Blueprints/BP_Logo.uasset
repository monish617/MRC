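; BP_Logo is an actor Blueprint that displays a selectable logo actor through its LogoClass child actor component.
; The construction script applies MyLogoClass to that component and records it as MyLogoClassSelected.
; Tick compares the two variables and, when they differ, runs the same update through a DoOnce gate that resets afterward, so class changes at runtime also swap the logo.
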(event Custom|UpdateLogo
  (ChildActorComponent|SetChildActorClass (Variables|Default|GetLogoClass) (Variables|Control|GetMyLogoClass))
  (Variables|Control|SetMyLogoClassSelected (Variables|Control|GetMyLogoClass))
  (CallFunction|ResetClassCheck))

(event Custom|ResetClassCheck
  (Utilities|FlowControl|DoOnce false) ; enters at Reset
)

(event Custom|CheckLogoClass
  (if (not (== (Variables|Control|GetMyLogoClass) (Variables|Control|GetMyLogoClassSelected)))
    (Utilities|FlowControl|DoOnce false
      (:Completed
        (CallFunction|UpdateLogo)))))

(event EventTick
  (params (DeltaSeconds :type Float%20%28single-precision%29))
  (CallFunction|CheckLogoClass))

(fn ConstructionScript
  (CallFunction|UpdateLogo))