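; Team victory bump controller that pulls the team name from the hype chamber controller for the victory scene's text assets.
; UpdateText runs on construction and from Tick after a short delay, copying TeamAName from each BP_HypeChamber_Controller in the level into TeamName.
; The text side is unfinished: the TeamNameAssets loop only checks validity, SetText is empty, and the uppercase conversion is unused.
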(event Custom|UpdateText
  (Utilities|FlowControl|Sequence
    (:then_0
      (for _array_element (Variables|Default|GetTeamNameAssets)
        (Utilities|IsValid _array_element)))
    (:then_1
      (bind _outactors (Actor|GetAllActorsOfClass "/Game/EsportsSample/_ArtistElements/Blueprints/BP_HypeChamber_Controller.BP_HypeChamber_Controller_C"))
      (for _array_element_2 _outactors
        (Utilities|IsValid _array_element_2
          (:Is%20Valid
            (Variables|Default|SetTeamName (Variables|/Game/EsportsSample/_ArtistElements/Blueprints/BP_HypeChamber_Controller.BP_HypeChamber_Controller_C|GetTeamAName _array_element_2))))))))

(event EventBeginPlay)

(event EventTick
  (params (DeltaSeconds :type Float%20%28single-precision%29))
  (Utilities|FlowControl|Delay 0.01)
  (CallFunction|UpdateText))

(fn ConstructionScript
  (CallFunction|UpdateText))