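; Artist-built platform actor for the esports sample, posed by rotating twelve hinge components and a center piece.
; The Construction Script adds HingeRotate as local roll to each hinge and PlatformCenterRotate as local yaw to the center.
; BeginPlay repeats the same relative rotations, adding them again at game start; nothing animates per frame.
; A secondary-platform visibility toggle is present but never runs.
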(event EventBeginPlay
  ;[0 0 0] Rotate Hinges
  (for _array_element (Utilities|Array|MakeArray (Variables|Default|GetHinge8) (Variables|Default|GetHinge2) (Variables|Default|GetHinge11) (Variables|Default|GetHinge9) (Variables|Default|GetHinge10) (Variables|Default|GetHinge7) (Variables|Default|GetHinge1) (Variables|Default|GetHinge5) (Variables|Default|GetHinge6) (Variables|Default|GetHinge3) (Variables|Default|GetHinge4) (Variables|Default|GetHinge12))
    (Transformation|AddLocalRotation _array_element (Math|Rotator|MakeRotator (Variables|Default|GetHinge%20Rotate) 0.0 0.0) false false))
  ;[0 0 0] Rotate Center
  (Transformation|AddLocalRotation (Variables|Default|GetPlatform_Center) (Math|Rotator|MakeRotator 0.0 0.0 (Variables|Default|GetPlatform%20Center%20Rotate)) false false))

(event Collision|EventActorBeginOverlap
  (params (OtherActor :type Actor%20Object%20Reference)))

(event EventTick
  (params (DeltaSeconds :type Float%20%28single-precision%29)))

(fn ConstructionScript
  ;[0 0 0] Rotate Hinges
  (for _array_element (Utilities|Array|MakeArray (Variables|Default|GetHinge8) (Variables|Default|GetHinge2) (Variables|Default|GetHinge11) (Variables|Default|GetHinge9) (Variables|Default|GetHinge10) (Variables|Default|GetHinge7) (Variables|Default|GetHinge1) (Variables|Default|GetHinge5) (Variables|Default|GetHinge6) (Variables|Default|GetHinge3) (Variables|Default|GetHinge4) (Variables|Default|GetHinge12))
    (Transformation|AddLocalRotation _array_element (Math|Rotator|MakeRotator (Variables|Default|GetHinge%20Rotate) 0.0 0.0) false false))
  ;[0 0 0] Rotate Center
  (Transformation|AddLocalRotation (Variables|Default|GetPlatform_Center) (Math|Rotator|MakeRotator 0.0 0.0 (Variables|Default|GetPlatform%20Center%20Rotate)) false false))