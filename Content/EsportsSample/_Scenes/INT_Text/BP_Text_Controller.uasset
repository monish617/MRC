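; Text controller for the esports sample's Hype Chamber that mirrors the text settings of BP_HypeChamber_Controller.
; UpdateText runs on construction and from Tick through a short Delay, finding the controller and caching its layout version.
; It stores the first line, appending the second for non-empty double-line layouts.
; Code for repositioning and Text3D output is disconnected, so the live graph only updates variables.
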(event Custom|UpdateText
  (Utilities|FlowControl|Sequence
    (:then_0
      (bind _outactors (Actor|GetAllActorsOfClass "/Game/EsportsSample/_ArtistElements/Blueprints/BP_HypeChamber_Controller.BP_HypeChamber_Controller_C"))
      (for _array_element _outactors
        (bind _output_get (Variables|Default|SetController _array_element))
        (Utilities|IsValid _output_get
          (:Is%20Valid
            (Variables|Default|SetMyTextVer (Variables|/Game/EsportsSample/_ArtistElements/Blueprints/BP_HypeChamber_Controller.BP_HypeChamber_Controller_C|GetTextVer _output_get))
            (if (Utilities|Select :Index (Variables|Default|GetMyTextVer) :NewEnumerator0 false :NewEnumerator1 true :NewEnumerator2 false :NewEnumerator3 true)
              (if (> (Utilities|String|Len (Variables|/Game/EsportsSample/_ArtistElements/Blueprints/BP_HypeChamber_Controller.BP_HypeChamber_Controller_C|GetTextLine2 _output_get)) 0)
                (Variables|Default|SetTextLine1 (Utilities|String|Append (Variables|/Game/EsportsSample/_ArtistElements/Blueprints/BP_HypeChamber_Controller.BP_HypeChamber_Controller_C|GetTextLine1 _output_get) " 
" (Variables|/Game/EsportsSample/_ArtistElements/Blueprints/BP_HypeChamber_Controller.BP_HypeChamber_Controller_C|GetTextLine2 _output_get)))
                (else
                  (Variables|Default|SetTextLine1 (Variables|/Game/EsportsSample/_ArtistElements/Blueprints/BP_HypeChamber_Controller.BP_HypeChamber_Controller_C|GetTextLine1 _output_get) :!label _label)
                  (Variables|Default|SetOffset (Utilities|Select :Index (Variables|Default|GetMyTextVer) :NewEnumerator0 "0, 0, 0" :NewEnumerator1 "0, 0, 0" :NewEnumerator2 "0, 0, 0" :NewEnumerator3 "0, 0, 0"))))
              (else
                (goto _label)))))))
    (:then_1
      (Variables|Default|GetController
        (:then)
        (:else)))
    (:then_2
      (Variables|Default|GetController
        (:then)
        (:else)))))

(event EventBeginPlay)

(event EventTick
  (params (DeltaSeconds :type Float%20%28single-precision%29))
  (Utilities|FlowControl|Delay 0.01)
  (CallFunction|UpdateText))

(fn ConstructionScript
  (CallFunction|UpdateText))