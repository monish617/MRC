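; BP_CornerScreen is an esports-sample art prop: a corner screen with separately configurable left and right screen images.
; Its construction script creates dynamic instances of regular and bright left/right corner screen materials, feeding the left and right texture variables into each emissive map.
; These instances go onto the screen slots of the CornerScreenRegular and CornerScreenBright components, so both versions show the same images.
; The event graph holds no active logic.
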(event EventBeginPlay)

(event Collision|EventActorBeginOverlap
  (params (OtherActor :type Actor%20Object%20Reference)))

(event EventTick
  (params (DeltaSeconds :type Float%20%28single-precision%29)))

(fn ConstructionScript
  ;[0 0 0] Right
  (bind _returnvalue (Rendering|Material|CreateDynamicMaterialInstance "/Game/EsportsSample/_ArtistElements/Materials/Screens/MI_Screen_CornerR.MI_Screen_CornerR" "None" "None" :!class /Script/Engine.KismetMaterialLibrary))
  (Rendering|Material|SetTextureParameterValue _returnvalue "Emmisive Map" (Variables|Default|GetScreen%20Texture%20Right))
  (Rendering|Material|SetMaterial (Variables|Default|GetCornerScreen_Regular) 3 _returnvalue)
  ;[0 0 0] Left
  (bind _returnvalue_2 (Rendering|Material|CreateDynamicMaterialInstance "/Game/EsportsSample/_ArtistElements/Materials/Screens/MI_Screen_CornerL.MI_Screen_CornerL" "None" "None" :!class /Script/Engine.KismetMaterialLibrary))
  (Rendering|Material|SetTextureParameterValue _returnvalue_2 "Emmisive Map" (Variables|Default|GetScreen%20Texture%20Left))
  (Rendering|Material|SetMaterial (Variables|Default|GetCornerScreen_Regular) 4 _returnvalue_2)
  ;[0 0 0] Right_Bright
  (bind _returnvalue_3 (Rendering|Material|CreateDynamicMaterialInstance "/Game/EsportsSample/_ArtistElements/Materials/Screens/MI_Screen_CornerR_Bright.MI_Screen_CornerR_Bright" "None" "None" :!class /Script/Engine.KismetMaterialLibrary))
  (Rendering|Material|SetTextureParameterValue _returnvalue_3 "Emmisive Map" (Variables|Default|GetScreen%20Texture%20Right))
  (Rendering|Material|SetMaterial (Variables|Default|GetCornerScreen_Bright) 3 _returnvalue_3)
  ;[0 0 0] Left_Bright
  (bind _returnvalue_4 (Rendering|Material|CreateDynamicMaterialInstance "/Game/EsportsSample/_ArtistElements/Materials/Screens/MI_Screen_CornerL_Bright.MI_Screen_CornerL_Bright" "None" "None" :!class /Script/Engine.KismetMaterialLibrary))
  (Rendering|Material|SetTextureParameterValue _returnvalue_4 "Emmisive Map" (Variables|Default|GetScreen%20Texture%20Left))
  (Rendering|Material|SetMaterial (Variables|Default|GetCornerScreen_Bright) 4 _returnvalue_4))