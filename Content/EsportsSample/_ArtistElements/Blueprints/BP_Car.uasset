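; BP_Car is a wrapper actor that displays a selectable car class through a child actor component.
; The construction script applies the chosen class, and Tick watches for changes, using a resettable DoOnce to rebuild the child when the selection differs.
; After each update it casts the child to BP_Car_Base and caches its mesh, systematic flag, body paint material ID and two slot materials.
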(event Custom|UpdateCar
  (ChildActorComponent|SetChildActorClass (Variables|Default|GetCarClass) (Variables|Default|GetMyCarClass))
  (Variables|Default|SetMyCarClassSelected (Variables|Default|GetMyCarClass))
  (CallFunction|ResetClassCheck)
  (CallFunction|SetChildSettings))

(event Custom|ResetClassCheck
  (Utilities|FlowControl|DoOnce false) ; enters at Reset
)

(event Custom|CheckCarClass
  (if (not (== (Variables|Default|GetMyCarClass) (Variables|Default|GetMyCarClassSelected)))
    (Utilities|FlowControl|DoOnce false
      (:Completed
        (CallFunction|UpdateCar)))))

(event Custom|SetChildSettings
  (bind _carclass (Variables|Default|GetCarClass))
  (bind _childactor (Variables|/Script/Engine.ChildActorComponent|GetChildActor _carclass))
  (Utilities|IsValid _childactor
    (:Is%20Valid
      (bind _asbp_car_base (Utilities|Casting|CastToBP_Car_Base _childactor))
      (Utilities|IsValid (Variables|/Game/EsportsSample/_ArtistElements/Blueprints/Cars/BP_Car_Base.BP_Car_Base_C|GetSM_Car _asbp_car_base)
        (:Is%20Valid
          (bind _output_get (Variables|Default|SetMyCarMesh (Variables|/Game/EsportsSample/_ArtistElements/Blueprints/Cars/BP_Car_Base.BP_Car_Base_C|GetSM_Car _asbp_car_base)))
          (Variables|Default|SetisSystematic (Variables|/Game/EsportsSample/_ArtistElements/Blueprints/Cars/BP_Car_Base.BP_Car_Base_C|GetisSystematic _asbp_car_base))
          (Variables|Default|SetBody%20Paint%20Mat%20ID (Variables|/Game/EsportsSample/_ArtistElements/Blueprints/Cars/BP_Car_Base.BP_Car_Base_C|GetBodyPaintMatID _asbp_car_base))
          (Variables|Default|SetSlot0Material (Rendering|Material|GetMaterial _output_get 0))
          (Variables|Default|SetSlot3Material (Rendering|Material|GetMaterial _output_get 3)))))))

(event EventTick
  (params (DeltaSeconds :type Float%20%28single-precision%29))
  (CallFunction|CheckCarClass))

(fn ConstructionScript
  (CallFunction|UpdateCar))