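; BP_TeamLight is a spotlight actor for the esports sample that lights in the color of its assigned team.
; Exposed variables set intensity, cone angles, attenuation, ray-tracing samples, visibility, shadows and lighting channels.
; The Team enum selects the TeamALight or TeamBLight vector from the MPC_TeamColorController parameter collection as the light color.
; Identical logic runs in the Construction Script and on BeginPlay, applying settings both at construction and when play starts.
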(event EventBeginPlay
  (bind _spotlight (Variables|Default|GetSpotLight))
  (Rendering|Components|Light|SetIntensity _spotlight (Variables|LightProperties|GetLight%20Intensity))
  (Rendering|Lighting|SetInnerConeAngle _spotlight (Variables|LightProperties|GetInner%20Cone%20Angle))
  (Rendering|Lighting|SetOuterConeAngle _spotlight (Variables|LightProperties|GetOuter%20Cone%20Angle))
  (Class|LightComponentBase|SetSamplesPerPixel _spotlight (Variables|LightProperties|GetRayTrace%20SamplesPerPixel))
  (Rendering|SetVisibility _spotlight (Variables|LightProperties|GetVisibility) true)
  (Rendering|Components|Light|SetCastShadows _spotlight (Variables|LightProperties|GetCast%20Shadows))
  (Rendering|Lighting|SetAttenuationRadius _spotlight (Variables|LightProperties|GetAttenuation%20Radius))
  (Rendering|Components|SetLightingChannels _spotlight (Variables|LightProperties|GetLighting%20Channel%200) (Variables|LightProperties|GetLighting%20Channel%201) (Variables|LightProperties|GetLighting%20Channel%202))
  (if (Utilities|Enum|Equal(Enum) (Variables|Default|GetTeam) "NewEnumerator0")
    (bind _returnvalue (Rendering|Material|GetVectorParameterValue "/Game/EsportsSample/_ArtistElements/Materials/Collections/MPC_TeamColorController.MPC_TeamColorController" "TeamALight" :!class /Script/Engine.KismetMaterialLibrary))
    (Rendering|Components|Light|SetLightColor _spotlight _returnvalue true)
    (else
      (bind _returnvalue_2 (Rendering|Material|GetVectorParameterValue "/Game/EsportsSample/_ArtistElements/Materials/Collections/MPC_TeamColorController.MPC_TeamColorController" "TeamBLight" :!class /Script/Engine.KismetMaterialLibrary))
      (Rendering|Components|Light|SetLightColor _spotlight _returnvalue_2 true))))

(fn ConstructionScript
  (bind _spotlight (Variables|Default|GetSpotLight))
  (Rendering|Components|Light|SetIntensity _spotlight (Variables|LightProperties|GetLight%20Intensity))
  (Rendering|Lighting|SetInnerConeAngle _spotlight (Variables|LightProperties|GetInner%20Cone%20Angle))
  (Rendering|Lighting|SetOuterConeAngle _spotlight (Variables|LightProperties|GetOuter%20Cone%20Angle))
  (Class|LightComponentBase|SetSamplesPerPixel _spotlight (Variables|LightProperties|GetRayTrace%20SamplesPerPixel))
  (Rendering|SetVisibility _spotlight (Variables|LightProperties|GetVisibility) true)
  (Rendering|Components|Light|SetCastShadows _spotlight (Variables|LightProperties|GetCast%20Shadows))
  (Rendering|Lighting|SetAttenuationRadius _spotlight (Variables|LightProperties|GetAttenuation%20Radius))
  (Rendering|Components|SetLightingChannels _spotlight (Variables|LightProperties|GetLighting%20Channel%200) (Variables|LightProperties|GetLighting%20Channel%201) (Variables|LightProperties|GetLighting%20Channel%202))
  (if (Utilities|Enum|Equal(Enum) (Variables|Default|GetTeam) "NewEnumerator0")
    (bind _returnvalue (Rendering|Material|GetVectorParameterValue "/Game/EsportsSample/_ArtistElements/Materials/Collections/MPC_TeamColorController.MPC_TeamColorController" "TeamALight" :!class /Script/Engine.KismetMaterialLibrary))
    (Rendering|Components|Light|SetLightColor _spotlight _returnvalue true)
    (else
      (bind _returnvalue_2 (Rendering|Material|GetVectorParameterValue "/Game/EsportsSample/_ArtistElements/Materials/Collections/MPC_TeamColorController.MPC_TeamColorController" "TeamBLight" :!class /Script/Engine.KismetMaterialLibrary))
      (Rendering|Components|Light|SetLightColor _spotlight _returnvalue_2 true))))